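; BP_Target is a shootable target actor that loses health when struck by first-person projectiles and counts toward the player's goal.
; On Hit, it consumes each BP_FirstPersonProjectile once via its DamageConsumed flag, destroys it, and subtracts fixed damage from Health.
; At zero health, a Destroyed flag guards a single kill that increments TargetsHit on BP_FirstPersonCharacter, calls CheckGoal, and destroys the target.
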(event EventBeginPlay)

(event Collision|EventActorBeginOverlap
  (params (OtherActor :type Actor%20Object%20Reference)))

(event EventTick
  (params (DeltaSeconds :type Float%20%28single-precision%29)))

(event Collision|EventHit
  (params (MyComp :type Primitive%20Component%20Object%20Reference) (Other :type Actor%20Object%20Reference) (OtherComp :type Primitive%20Component%20Object%20Reference) (bSelfMoved :type Boolean) (HitLocation :type Vector :default "0, 0, 0") (HitNormal :type Vector :default "0, 0, 0") (NormalImpulse :type Vector :default "0, 0, 0") (Hit :type Hit%20Result%20Structure%20%28by%20ref%29))
  (bind _asbp_first_person_projectile (Utilities|Casting|CastToBP_FirstPersonProjectile Other))
  (if (not (Variables|/Game/FirstPerson/Blueprints/BP_FirstPersonProjectile.BP_FirstPersonProjectile_C|GetbDamageConsumed _asbp_first_person_projectile))
    (Variables|/Game/FirstPerson/Blueprints/BP_FirstPersonProjectile.BP_FirstPersonProjectile_C|SetbDamageConsumed _asbp_first_person_projectile true)
    (Actor|DestroyActor _asbp_first_person_projectile)
    (if (not (Variables|Default|GetbDestroyed))
      (bind _output_get (Variables|Default|SetHealth (- (Variables|Default|GetHealth) 25)))
      (if (<= _output_get 0)
        (Variables|Default|SetbDestroyed true)
        (bind _asbp_first_person_character (Utilities|Casting|CastToBP_FirstPersonCharacter (Game|GetPlayerCharacter 0)))
        (Variables|/Game/FirstPerson/Blueprints/BP_FirstPersonCharacter.BP_FirstPersonCharacter_C|SetTargetsHit _asbp_first_person_character (+ (Variables|/Game/FirstPerson/Blueprints/BP_FirstPersonCharacter.BP_FirstPersonCharacter_C|GetTargetsHit _asbp_first_person_character) 1))
        (Default|CheckGoal _asbp_first_person_character)
        (Actor|DestroyActor)))))

(fn ConstructionScript)